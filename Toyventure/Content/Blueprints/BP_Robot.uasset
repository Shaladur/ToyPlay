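; BP_Robot is an interactable puzzle robot that takes three colored batteries from the player and ends the game once all are inserted.
; Its box overlap sets or clears itself as the character's Interactive target.
; Interact moves a matching battery from the player's BatteryInventory into an empty slot, hiding that color's cylinder.
; When IsEnigmaOver passes, EndGame plays a looping spin animation, then loads L_End after a delay.
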(event OnComponentBeginOverlap(Box)
  (params (OverlappedComponent :type Primitive%20Component%20Object%20Reference) (OtherActor :type Actor%20Object%20Reference) (OtherComp :type Primitive%20Component%20Object%20Reference) (OtherBodyIndex :type Integer) (bFromSweep :type Boolean) (SweepResult :type Hit%20Result%20Structure%20%28by%20ref%29))
  (bind _asbp_third_person_character (Utilities|Casting|CastToBP_ThirdPersonCharacter OtherActor))
  (Variables|/Game/ThirdPerson/Blueprints/BP_ThirdPersonCharacter.BP_ThirdPersonCharacter_C|SetInteractive _asbp_third_person_character self))

(event OnComponentEndOverlap(Box)
  (params (OverlappedComponent :type Primitive%20Component%20Object%20Reference) (OtherActor :type Actor%20Object%20Reference) (OtherComp :type Primitive%20Component%20Object%20Reference) (OtherBodyIndex :type Integer))
  (bind _asbp_third_person_character (Utilities|Casting|CastToBP_ThirdPersonCharacter OtherActor))
  (Variables|/Game/ThirdPerson/Blueprints/BP_ThirdPersonCharacter.BP_ThirdPersonCharacter_C|SetInteractive _asbp_third_person_character 0))

(event Custom|EndGame
  (Transformation|SetRelativeRotation (Variables|Default|GetRobotMesh) "0, 0, 0" false false)
  (Components|Animation|PlayAnimation (Variables|Default|GetRobotMesh) "/Game/Fab/Robot/attackspin.attackspin" true)
  (Utilities|FlowControl|Delay 5.0)
  (Game|OpenLevel(byName) "L_End"))

(event EventInteract
  (bind _asbp_third_person_character (Utilities|Casting|CastToBP_ThirdPersonCharacter (Game|GetPlayerCharacter 0)))
  (bind _array_element (Utilities|Array|ForEachLoopwithBreak (Variables|/Game/ThirdPerson/Blueprints/BP_ThirdPersonCharacter.BP_ThirdPersonCharacter_C|GetbatteryInventory _asbp_third_person_character) :!label _label)
    (:LoopBody
      (switch Utilities|FlowControl|Switch|SwitchonE_Color _array_element
        (:NewEnumerator0
          (if (== (Variables|Default|GetIsBlueIn?) false)
            (Variables|Default|SetIsBlueIn? true)
            (Utilities|Array|RemoveItem (Variables|/Game/ThirdPerson/Blueprints/BP_ThirdPersonCharacter.BP_ThirdPersonCharacter_C|GetbatteryInventory _asbp_third_person_character) _array_element)
            (Rendering|SetVisibility (Variables|Default|GetBlueCylinder) false false)
            (goto _label Break)))
        (:NewEnumerator1
          (if (== (Variables|Default|GetIsGreenIn?) false)
            (Variables|Default|SetIsGreenIn? true)
            (Utilities|Array|RemoveItem (Variables|/Game/ThirdPerson/Blueprints/BP_ThirdPersonCharacter.BP_ThirdPersonCharacter_C|GetbatteryInventory _asbp_third_person_character) _array_element)
            (Rendering|SetVisibility (Variables|Default|GetgreenCylinder) false false)
            (goto _label Break)))
        (:NewEnumerator2
          (if (== (Variables|Default|GetIsOrangeIn?) false)
            (Variables|Default|SetIsOrangeIn? true)
            (Utilities|Array|RemoveItem (Variables|/Game/ThirdPerson/Blueprints/BP_ThirdPersonCharacter.BP_ThirdPersonCharacter_C|GetbatteryInventory _asbp_third_person_character) _array_element)
            (Rendering|SetVisibility (Variables|Default|GetOrangeCylinder) false false)
            (goto _label Break)))))
    (:Completed
      (if (Utilities|IsEnigmaOver?)
        (CallFunction|EndGame)))))

(fn ConstructionScript)