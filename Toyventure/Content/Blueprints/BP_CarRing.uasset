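; BP_CarRing is a numbered checkpoint ring for the sports car, where a ring with no NextRing reveals its battery.
; BeginPlay hides the linked Battery and disables its collision.
; On the car's first overlap, the ring plays a shutter sound and either disables its box (NextRing set) or reveals any Battery, then disables the box.
; The construction script writes Index onto the text render; its Index branch is empty.
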(event OnComponentBeginOverlap(Box)
  (params (OverlappedComponent :type Primitive%20Component%20Object%20Reference) (OtherActor :type Actor%20Object%20Reference) (OtherComp :type Primitive%20Component%20Object%20Reference) (OtherBodyIndex :type Integer) (bFromSweep :type Boolean) (SweepResult :type Hit%20Result%20Structure%20%28by%20ref%29))
  (Utilities|Casting|CastToSportsCar_Pawn OtherActor)
  (Utilities|FlowControl|DoOnce false
    (:Completed
      (Audio|PlaySoundatLocation "/Engine/VREditor/Sounds/UI/Camera_Shutter.Camera_Shutter" (Transformation|GetActorLocation) "0, 0, 0" 1.0 1.0 0.0 0 0 0 0)
      (Variables|Default|GetNextRing
        (:then
          _)
        (:else
          (bind _battery (Variables|Default|GetBattery)
            (:then
              (Collision|SetActorEnableCollision _battery true)
              (Rendering|SetVisibility (Variables|/Game/Blueprints/BP_Battery.BP_Battery_C|GetBatteryMesh _battery) true false))
            (:else))))
      (Collision|SetCollisionEnabled (Variables|Default|GetBox) "NoCollision"))))

(event EventBeginPlay
  (bind _battery (Variables|Default|GetBattery)
    (:then
      (Collision|SetActorEnableCollision _battery false)
      (Rendering|SetVisibility (Variables|/Game/Blueprints/BP_Battery.BP_Battery_C|GetBatteryMesh _battery) false false))
    (:else)))

(fn ConstructionScript
  (bind _index (Variables|Default|GetIndex))
  (if (!= _index 1)
    _
    (else
      _))
  (Rendering|Components|TextRender|SetText (Variables|Default|GetTextRender) (Utilities|Text|ToText(Integer) _index)))