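; BP_Battery is a colored battery pickup that the player collects into the character's battery inventory.
; The construction script sets the mesh material from its Color value.
; Overlapping its box registers it as the third-person character's Interactive target; Interact then clears that reference, adds its Color to BatteryInventory, plays a ping sound and destroys the actor.
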(event OnComponentBeginOverlap(Box)
  (params (OverlappedComponent :type Primitive%20Component%20Object%20Reference) (OtherActor :type Actor%20Object%20Reference) (OtherComp :type Primitive%20Component%20Object%20Reference) (OtherBodyIndex :type Integer) (bFromSweep :type Boolean) (SweepResult :type Hit%20Result%20Structure%20%28by%20ref%29))
  (bind _asbp_third_person_character (Utilities|Casting|CastToBP_ThirdPersonCharacter OtherActor))
  (Variables|/Game/ThirdPerson/Blueprints/BP_ThirdPersonCharacter.BP_ThirdPersonCharacter_C|SetInteractive _asbp_third_person_character self))

(event EventInteract
  (bind _asbp_third_person_character (Utilities|Casting|CastToBP_ThirdPersonCharacter (Game|GetPlayerCharacter 0)))
  (Variables|/Game/ThirdPerson/Blueprints/BP_ThirdPersonCharacter.BP_ThirdPersonCharacter_C|SetInteractive _asbp_third_person_character 0)
  (Utilities|Array|Add (Variables|/Game/ThirdPerson/Blueprints/BP_ThirdPersonCharacter.BP_ThirdPersonCharacter_C|GetbatteryInventory _asbp_third_person_character) (Variables|Default|GetColor))
  (Audio|PlaySoundatLocation "/Engine/EngineSounds/1kSineTonePing.1kSineTonePing" (Transformation|GetActorLocation) "0, 0, 0" 1.0 1.0 0.0 0 0 0 0)
  (Actor|DestroyActor))

(fn ConstructionScript
  (switch Utilities|FlowControl|Switch|SwitchonE_Color (Variables|Default|GetColor)
    (:NewEnumerator0
      (LocalVariables|SetMaterial "/AnimationSharing/AnimSharingBlue.AnimSharingBlue"))
    (:NewEnumerator1
      (LocalVariables|SetMaterial "/AnimationSharing/AnimSharingGreen.AnimSharingGreen"))
    (:NewEnumerator2
      (LocalVariables|SetMaterial "/Engine/TemplateResources/MI_Template_BaseOrange.MI_Template_BaseOrange")))
  (Rendering|Material|SetMaterial (Variables|Default|GetBatteryMesh) 1 (LocalVariables|GetMaterial)))